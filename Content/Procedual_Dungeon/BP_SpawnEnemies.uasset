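; BP_SpawnEnemies is an unfinished procedural-dungeon actor that reacts to overlaps, apparently intended to spawn enemies.
; On any overlap it calls SpawnActor with no class set and clears its SpawnEnemies variable.
; It then gathers all actors of the spawned actor's class into EnemyCount and prints the count only when it is zero.
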(event `self.ReceiveActorBeginOverlap`
  (params (OtherActor :type "Actor Object Reference"))
  (bind _returnvalue (`|SpawnActorFromClass` null (struct) "Undefined" "MultiplyWithRoot"))
  (set `self.Spawn_Enemies` _)
  (bind _outactors (`GameplayStatics.GetAllActorsOfClass` (`GameplayStatics.GetObjectClass` _returnvalue)))
  (bind _output_get (set `self.Enemy_Count` _outactors))
  (bind _output_get_2 (set `self.Numbers` (`KismetArrayLibrary.Array_Length` _output_get)))
  (if (== _output_get_2 0)
    (`KismetSystemLibrary.PrintString` (`KismetStringLibrary.Conv_IntToString` _output_get_2))))

(fn `UserConstructionScript`)