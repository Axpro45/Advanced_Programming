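; Dungeon room actor that generates a procedural layout by spawning copies of itself.
; On BeginPlay, a room with CanSpawn set repeatedly picks a random placed room and calls SpawnNewRoom, then runs DeleteWalls on all rooms.
; SpawnNewRoom uses sphere traces at four arrows to find free sides, re-rolling the random side separately for placement and flag updates.
; DeleteWalls repeats those traces and destroys walls where they hit.
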(event `self.ReceiveBeginPlay`
  ;[1 1 1] Begin Play
  (if (`self.CanSpawn?`)
    (`KismetArrayLibrary.Array_AddUnique` (`self.SpawnedRooms`) self)
    (for _ (range (+ (`self.Iterations`) 1))
      (bind _roomspawn (`self.SpawnNewRoom` (`KismetArrayLibrary.Array_Random` (`self.SpawnedRooms`))))
      (`KismetArrayLibrary.Array_AddUnique` (`self.SpawnedRooms`) _roomspawn))
    (for _array_element (`self.SpawnedRooms`)
      (`self.Delete Walls` _array_element))))

(event `Delete Walls`
  (bind _returnvalue (`SceneComponent.K2_GetComponentLocation` (`self.Right Arrow`)))
  (bind _returnvalue_2 (`SceneComponent.K2_GetComponentLocation` (`self.Front Arrow`)))
  (bind _returnvalue_3 (`SceneComponent.K2_GetComponentLocation` (`self.Back Arrow`)))
  (bind _returnvalue_4 (`SceneComponent.K2_GetComponentLocation` (`self.Left Arrow`)))
  ;[1 1 1 1 81] Delete walls
  (`|ExecutionSequence`
    (:`then_0`
      (bind (_outhits _returnvalue_5) (`KismetSystemLibrary.SphereTraceMulti` :`Start` _returnvalue_2 :`End` _returnvalue_2 :`Radius` 40.0 :`TraceChannel` "TraceTypeQuery1" :`DrawTime` 1.0))
      (if _returnvalue_5
        (`ActorComponent.K2_DestroyComponent` (`self.Front wall`))))
    (:`then_1`
      (bind (_outhits_2 _returnvalue_6) (`KismetSystemLibrary.SphereTraceMulti` :`Start` _returnvalue_3 :`End` _returnvalue_3 :`Radius` 40.0 :`TraceChannel` "TraceTypeQuery1" :`DrawTime` 1.0))
      (if _returnvalue_6
        (`ActorComponent.K2_DestroyComponent` (`self.Back wall`))))
    (:`then_2`
      (bind (_outhits_3 _returnvalue_7) (`KismetSystemLibrary.SphereTraceMulti` :`Start` _returnvalue_4 :`End` _returnvalue_4 :`Radius` 40.0 :`TraceChannel` "TraceTypeQuery1" :`DrawTime` 1.0))
      (if _returnvalue_7
        (`ActorComponent.K2_DestroyComponent` (`self.Left Wall`))))
    (:`then_3`
      (bind (_outhits_4 _returnvalue_8) (`KismetSystemLibrary.SphereTraceMulti` :`Start` _returnvalue :`End` _returnvalue :`Radius` 40.0 :`TraceChannel` "TraceTypeQuery1" :`DrawTime` 1.0))
      (if _returnvalue_8
        (`ActorComponent.K2_DestroyComponent` (`self.Right wall`))))))

(event `SetBooleans`
  (bind _returnvalue (`SceneComponent.K2_GetComponentLocation` (`self.Front Arrow`)))
  (bind _returnvalue_2 (`SceneComponent.K2_GetComponentLocation` (`self.Back Arrow`)))
  (bind _returnvalue_3 (`SceneComponent.K2_GetComponentLocation` (`self.Left Arrow`)))
  (bind _returnvalue_4 (`SceneComponent.K2_GetComponentLocation` (`self.Right Arrow`)))
  ;[1 0 0] Set Booleans
  (`|ExecutionSequence`
    (:`then_0`
      (bind (_outhits _returnvalue_5) (`KismetSystemLibrary.SphereTraceMulti` :`Start` _returnvalue :`End` _returnvalue :`Radius` 40.0 :`TraceChannel` "TraceTypeQuery1" :`DrawTime` 1.0))
      (if _returnvalue_5
        (`KismetArrayLibrary.Array_Set` (`self.FBLR_Spawn`) 0 true)))
    (:`then_1`
      (bind (_outhits_2 _returnvalue_6) (`KismetSystemLibrary.SphereTraceMulti` :`Start` _returnvalue_2 :`End` _returnvalue_2 :`Radius` 40.0 :`TraceChannel` "TraceTypeQuery1" :`DrawTime` 1.0))
      (if _returnvalue_6
        (`KismetArrayLibrary.Array_Set` (`self.FBLR_Spawn`) 1 true)))
    (:`then_2`
      (bind (_outhits_3 _returnvalue_7) (`KismetSystemLibrary.SphereTraceMulti` :`Start` _returnvalue_3 :`End` _returnvalue_3 :`Radius` 40.0 :`TraceChannel` "TraceTypeQuery1" :`DrawTime` 1.0))
      (if _returnvalue_7
        (`KismetArrayLibrary.Array_Set` (`self.FBLR_Spawn`) 2 true)))
    (:`then_3`
      (bind (_outhits_4 _returnvalue_8) (`KismetSystemLibrary.SphereTraceMulti` :`Start` _returnvalue_4 :`End` _returnvalue_4 :`Radius` 40.0 :`TraceChannel` "TraceTypeQuery1" :`DrawTime` 1.0))
      (if _returnvalue_8
        (`KismetArrayLibrary.Array_Set` (`self.FBLR_Spawn`) 3 true)))))

(fn `SpawnNewRoom`
  (returns (RoomSpawn :type "/Game/Procedual_Dungeon/BP_dungeon Object Reference"))
  (bind _outitem (`KismetArrayLibrary.Array_Random` (`self.Indexes`)))
  (`KismetArrayLibrary.Array_Clear` (`self.Indexes`))
  (`self.SetBooleans`)
  (for (_array_element _array_index) (`self.FBLR_Spawn`)
    (if (not _array_element)
      (`KismetArrayLibrary.Array_AddUnique` (`self.Indexes`) _array_index)))
  (if (> (`KismetArrayLibrary.Array_Length` (`self.Indexes`)) 0)
    (bind _returnvalue (`|SpawnActorFromClass` "BP_dungeon_C" (`KismetMathLibrary.Conv_VectorToTransform` (+ (`SceneComponent.K2_GetComponentLocation` (`self.Arrow`)) (`|GetArrayItem` (`self.SpawnLocations`) _outitem))) "Undefined" "MultiplyWithRoot" null null))
    (`KismetArrayLibrary.Array_Set` (`self.FBLR_Spawn`) _outitem true)
    (switch `int` _outitem
      (:`0`
        (bind _fblr_spawn (`/Game/Procedual_Dungeon/BP_dungeon.FBLR_Spawn` _returnvalue))
        (`KismetArrayLibrary.Array_Set` _fblr_spawn 1 true))
      (:`1`
        (`KismetArrayLibrary.Array_Set` _fblr_spawn 0 true))
      (:`2`
        (`KismetArrayLibrary.Array_Set` _fblr_spawn 3 true))
      (:`3`
        (`KismetArrayLibrary.Array_Set` _fblr_spawn 2 true)))
    (return _returnvalue)
    (else
      (return self))))

(fn `UserConstructionScript`)